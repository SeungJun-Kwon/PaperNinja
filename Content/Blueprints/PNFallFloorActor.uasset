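; PNFallFloorActor is a floor that falls after the player pawn touches its trigger, then resets.
; An overlap on BoxTrigger by player pawn 0 waits briefly, then enables physics simulation on IronFloor.
; After a longer delay, physics is switched off and IronFloor moves to a hardcoded world transform rather than a saved starting one.
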(event `self.BoxTrigger.OnComponentBeginOverlap`
  (params (OverlappedComponent :type "PrimitiveComponent Object Reference") (OtherActor :type "Actor Object Reference") (OtherComp :type "PrimitiveComponent Object Reference") (OtherBodyIndex :type Integer) (bFromSweep :type Boolean) (SweepResult :type "HitResult Structure (by ref)"))
  (bind _ironfloor (`self.IronFloor`))
  (if (== OtherActor (`GameplayStatics.GetPlayerPawn` 0))
    (`KismetSystemLibrary.Delay` 1.0)
    (`PrimitiveComponent.SetSimulatePhysics` (`self.IronFloor`) true)
    (`KismetSystemLibrary.Delay` 5.0)
    (`PrimitiveComponent.SetSimulatePhysics` _ironfloor false)
    (`SceneComponent.K2_SetWorldTransform` _ironfloor (`KismetMathLibrary.MakeTransform` (250.0 350.0 10.0) (struct) (0.9 0.9 0.5)) false false)))

(fn `UserConstructionScript`)