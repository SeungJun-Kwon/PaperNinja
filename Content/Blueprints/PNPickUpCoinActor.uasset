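; Coin pickup actor that adds one coin to the overlapping PNPlayerPawn, then destroys itself.
; A timeline spins the mesh in yaw, while a half-second timer opens a gate that holds back box trigger overlaps until then.
; The audio component is added after the destroy call.
; A separate sequence branch spawns the pickup particle effect for actors tagged Player.
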(event `self.ReceiveBeginPlay`
  (`KismetSystemLibrary.K2_SetTimerDelegate` (delegate `EnablePickup`) 0.5)
  (bind (_direction _coinyaw) (`Timeline|CoinRotationTimeline`)
    (:`Update`
      (`SceneComponent.K2_SetRelativeRotation` (`self.Mesh`) (`KismetMathLibrary.MakeRotator` 0.0 0.0 _coinyaw) false false))))

(event `EnablePickup`
  (goto _label :!via `Open`))

(event `self.BoxTrigger.OnComponentBeginOverlap`
  (params (OverlappedComponent :type "PrimitiveComponent Object Reference") (OtherActor :type "Actor Object Reference") (OtherComp :type "PrimitiveComponent Object Reference") (OtherBodyIndex :type Integer) (bFromSweep :type Boolean) (SweepResult :type "HitResult Structure (by ref)"))
  (`/Engine/EditorBlueprintResources/StandardMacros.Gate` true :!label _label
    (:`Exit`
      (`|ExecutionSequence`
        (:`then_0`
          (bind _aspnplayer_pawn (cast `/Game/Blueprints/PNPlayerPawn` OtherActor))
          (`/Game/Blueprints/PNPlayerPawn.AddCoin` _aspnplayer_pawn 1)
          (`self.K2_DestroyActor`)
          (`AddComponent|NODE_AddAudioComponent-0`))
        (:`then_1`
          (if (`self.ActorHasTag` OtherActor "Player")
            (`GameplayStatics.SpawnEmitterAtLocation` "/Game/Particles/PS_PickUp_Coin.PS_PickUp_Coin" (`self.K2_GetActorLocation`))))))))

(fn `UserConstructionScript`)