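; PNSwitchActor is a switch that presses down when something overlaps its box trigger and releases when the overlap ends or TurnOff is called.
; A timeline lowers the mesh slightly and reverses to raise it, calling OnTurnedOn or OnTurnedOff when it finishes.
; IsMomentary serves as the pressed-state flag guarding both overlap events.
; TextRenderVisibleToggle matches the text's visibility to that flag.
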(event `self.BoxTrigger.OnComponentBeginOverlap`
  (params (OverlappedComponent :type "PrimitiveComponent Object Reference") (OtherActor :type "Actor Object Reference") (OtherComp :type "PrimitiveComponent Object Reference") (OtherBodyIndex :type Integer) (bFromSweep :type Boolean) (SweepResult :type "HitResult Structure (by ref)"))
  (if (not (`self.IsMomentary`))
    (set `self.IsMomentary` true)
    (bind (_direction _alpha) (`Timeline|SwitchTimeline` :!label _label)
      (:`Update`
        (`SceneComponent.K2_SetRelativeLocation` (`self.Mesh`) (`KismetMathLibrary.VLerp` (0.0 0.0 0.0) (0.0 0.0 -8.0) _alpha) false false))
      (:`Finished`
        (switch `ETimelineDirection` _direction
          (:`Forward`
            (`self.OnTurnedOn`))
          (:`Backward`
            (`self.OnTurnedOff`)))))))

(event `TurnOff`
  (set `self.IsMomentary` false :!label _label_2)
  (goto _label :!via `Reverse`))

(event `self.BoxTrigger.OnComponentEndOverlap`
  (params (OverlappedComponent :type "PrimitiveComponent Object Reference") (OtherActor :type "Actor Object Reference") (OtherComp :type "PrimitiveComponent Object Reference") (OtherBodyIndex :type Integer))
  (if (`self.IsMomentary`)
    (goto _label_2)))

(fn `TextRenderVisibleToggle`
  (`SceneComponent.SetVisibility` (`self.TextRender`) (`self.IsMomentary`) false))

(fn `UserConstructionScript`)