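; Game mode that respawns the player pawn when it is destroyed and handles background music.
; BeginPlay binds the respawn handler to the first pawn's OnDestroyed and starts the Bgm02 cue.
; The handler spawns a new PNPlayerPawn at a player start, possesses it, rebinds itself to that pawn and restarts the music.
; PlayBGM stops the MusicSpeaker, swaps its sound and plays from the beginning.
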(event `self.ReceiveBeginPlay`
  (add `self.OnDestroyed` (`GameplayStatics.GetPlayerPawn` 0) (delegate `RespanwPlayer`))
  (`self.PlayBGM` "/Game/Audios/SoundCue/bgm02_Cue.bgm02_Cue"))

(event `RespanwPlayer` :!signature `self.OnDestroyed`
  (params (DestroyedActor :type "Actor Object Reference"))
  (bind _returnvalue (`|SpawnActorFromClass` "/Game/Blueprints/PNPlayerPawn.PNPlayerPawn_C" (`self.GetTransform` (`self.K2_FindPlayerStart` null)) "Undefined" "OverrideRootScale" null null))
  (`Controller.Possess` (`GameplayStatics.GetPlayerController` 0) _returnvalue)
  (add `self.OnDestroyed` _returnvalue (delegate `RespanwPlayer`))
  (`self.PlayBGM` "/Game/Audios/SoundCue/bgm02_Cue.bgm02_Cue"))

(fn `PlayBGM`
  (params (NewBGM :type "SoundCue Object Reference"))
  (bind _musicspeaker (`self.MusicSpeaker`))
  (`AudioComponent.Stop` _musicspeaker)
  (`AudioComponent.SetSound` _musicspeaker NewBGM)
  (`AudioComponent.Play` (`self.MusicSpeaker`) 0.0))

(fn `UserConstructionScript`)